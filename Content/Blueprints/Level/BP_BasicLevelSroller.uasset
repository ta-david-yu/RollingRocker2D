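; Level scroller actor that drives auto-scrolling through a ScrollActorLocationOnMoveForward component and eases it to a halt on game over.
; It listens for the player state's GameOver change and starts a Tween, whose progress lowers the scroll speed multiplier from one toward zero.
; Debug logic prints the current scroll speed every tick, labeled as a multiplier, and lets Add and Subtract keys step that speed.
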(event `self.ReceiveBeginPlay`
  (bind _returnvalue (`GameplayStatics.GetPlayerController` 0))
  ;[1 1 1] Register Tween Update
  (add `TweenComponent.OnTweenUpdate` (`self.Tween`) (delegate `CustomEvent_0`))
  ;[1 1 1] Register Game Over State Handling
  (bind _asin_game_player_state (cast `InGamePlayerState` (`Controller.PlayerState` _returnvalue)))
  (add `InGamePlayerState.OnStateChanged` _asin_game_player_state (delegate `OnStateChanged_Event_0`))
  (`self.EnableInput` _returnvalue))

(event `OnStateChanged_Event_0`
  (params (prevState :type "EPlayerState Enum" :default "Normal") (newState :type "EPlayerState Enum" :default "Normal"))
  ;[1 1 1] Register Game Over State Handling
  (if (`|EnumEquality` newState "GameOver")
    (`TweenComponent.Tween` (`self.Tween`))))

(event `CustomEvent_0`
  (params (progress :type "Float (single-precision)"))
  ;[1 1 1] Register Tween Update
  (`self.HandleOnTweenUpdate` progress))

(event `self.ReceiveTick`
  (params (DeltaSeconds :type "Float (single-precision)"))
  (`KismetSystemLibrary.PrintText` (`KismetTextLibrary.Conv_StringToText` (`KismetStringLibrary.Concat_StrStr` "ScrollSpeedMultiplier: " (`KismetStringLibrary.Conv_DoubleToString` (`ScrollActorLocationOnMoveForward.m_CurrentAutoScrollSpeed` (`self.ScrollActorLocationOnMoveForward`))))) true false (struct :`G` 0.66 :`B` 1.0 :`A` 1.0) 0.0))

(event `Key|Add`
  (params (Key :type "Key Structure"))
  (bind _scrollactorlocationonmoveforward (`self.ScrollActorLocationOnMoveForward`))
  (:`Pressed`
    (set `ScrollActorLocationOnMoveForward.m_CurrentAutoScrollSpeed` (+ 1.0 (`ScrollActorLocationOnMoveForward.m_CurrentAutoScrollSpeed` _scrollactorlocationonmoveforward)) _scrollactorlocationonmoveforward)))

(event `Key|Subtract`
  (params (Key :type "Key Structure"))
  (bind _scrollactorlocationonmoveforward (`self.ScrollActorLocationOnMoveForward`))
  (:`Pressed`
    (set `ScrollActorLocationOnMoveForward.m_CurrentAutoScrollSpeed` (+ -1.0 (`ScrollActorLocationOnMoveForward.m_CurrentAutoScrollSpeed` _scrollactorlocationonmoveforward)) _scrollactorlocationonmoveforward)))

(fn `HandleOnTweenUpdate`
  (params (progress :type "Float (double-precision)"))
  (set `ScrollActorLocationOnMoveForward.m_AutoScrollSpeedMultiplier` (- 1.0 progress) (`self.ScrollActorLocationOnMoveForward`)))

(fn `UserConstructionScript`)