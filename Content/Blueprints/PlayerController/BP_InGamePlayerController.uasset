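; In-game player controller that drives a RollingRockerPawn's Rocker and Rod components from player input.
; On possession it caches the pawn, Rocker and Rod.
; An action toggles the Rocker between Free and Constrained movement, unless its state is External.
; In Free state a horizontal axis moves the Rocker directly; otherwise two axes move the Rod's left and right ends independently.
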(event `self.ReceivePossess`
  (params (PossessedPawn :type "Pawn Object Reference"))
  (bind _asrolling_rocker_pawn (cast `RollingRockerPawn` PossessedPawn))
  (bind _output_get (set `self._RollingRockerPawn` _asrolling_rocker_pawn))
  (set `self._Rocker` (`RollingRockerPawn.Rocker` _output_get))
  (set `self._Rod` (`RollingRockerPawn.Rod` _output_get)))

(event `InputAction|ActivateFreeMoveMode`
  (params (Key :type "Key Structure"))
  (:`Pressed`
    (if (not (`Rocker.IsMovementState` (`self._Rocker`) "External"))
      (`Rocker.SetMovementState` (`self._Rocker`) (select `bool` (`Rocker.IsMovementState` (`self._Rocker`) "Free") :`false` "Free" :`true` "Constrained" :!type "ERockerMovementState Enum")))))

(event `InputAxis|FreeMoveHorizontal`
  (params (AxisValue :type "Float (single-precision)"))
  (if (`Rocker.IsMovementState` (`self._Rocker`) "Free")
    (`Rocker.FreeMove` (`self._Rocker`) AxisValue)))

(event `InputAxis|MoveRodLeftEnd`
  (params (AxisValue :type "Float (single-precision)"))
  (if (not (`Rocker.IsMovementState` (`self._Rocker`) "Free"))
    (`Rod.MoveLeftEnd` (`self._Rod`) AxisValue)))

(event `InputAxis|MoveRodRightEnd`
  (params (AxisValue :type "Float (single-precision)"))
  (if (not (`Rocker.IsMovementState` (`self._Rocker`) "Free"))
    (`Rod.MoveRightEnd` (`self._Rod`) AxisValue)))

(fn `UserConstructionScript`)