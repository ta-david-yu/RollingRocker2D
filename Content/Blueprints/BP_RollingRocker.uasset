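; BP_RollingRocker is a Blueprint with a Rod component whose line it previews through debug drawing.
; Its EditorTick event calls a function that draws a short-lived yellow debug line centered on the Rod.
; The endpoints come from rotating the Rod's forward vector by its Angle around the world negative Y axis and extending half its MLength each way.
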(event `/Game/Blueprints/Utility/BPI_EditorTick.EditorTick`
  (`self.On Draw Debug Rod Line`))

(fn `On Draw Debug Rod Line`
  (locals (rodCenter :type "Vector Structure" :default (0.0 0.0 0.0)))
  (bind _rod (`self.Rod`))
  (bind _returnvalue (* (`KismetMathLibrary.RotateAngleAxis` (`SceneComponent.GetForwardVector` _rod) (`Rod.Angle` _rod) (0.0 -1.0 0.0)) (/ (`Rod.m_Length` _rod) 2.0)))
  (bind _output_get (set `local.rodCenter` (`SceneComponent.K2_GetComponentLocation` _rod)))
  (`KismetSystemLibrary.DrawDebugLine` (+ _output_get _returnvalue) (- _output_get _returnvalue) (struct :`R` 1.0 :`G` 0.808609 :`A` 1.0) 0.2 0.5))

(fn `UserConstructionScript`)