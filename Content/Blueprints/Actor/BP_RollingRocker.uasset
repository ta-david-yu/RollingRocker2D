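; BP_RollingRocker is the player pawn: a sphere rocker that rolls on a tiltable rod and can fall and respawn.
; Construction wires RockerComponent to the rod and collision sphere, and hands the rod to RodAnimationController.
; On possession it binds to the player state's lives count, which drives the dots on its LivesUIWidget.
; Debug graphs draw the rod and its end ranges in editor tick, print motion values, and map test keys.
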(event `/Game/Blueprints/Utility/BPI_EditorTick.EditorTick`
  (`self.OnDrawDebugRod`))

(event `self.ReceiveTick`
  (params (DeltaSeconds :type "Float (single-precision)"))
  (`KismetSystemLibrary.PrintText` (`KismetTextLibrary.Conv_StringToText` (`KismetStringLibrary.Concat_StrStr` "Current Velocity: " (`KismetStringLibrary.Conv_DoubleToString` (`Rocker.m_CurrentVelocity` (`self.RockerComponent`))))) true false (struct :`G` 0.66 :`B` 1.0 :`A` 1.0) 0.0)
  (`KismetSystemLibrary.PrintText` (`KismetTextLibrary.Conv_StringToText` (`KismetStringLibrary.Concat_StrStr` "Gravity: " (`KismetStringLibrary.Conv_DoubleToString` (`Rocker.m_OnRodGravity` (`self.RockerComponent`))))) true false (struct :`G` 0.66 :`B` 1.0 :`A` 1.0) 0.0)
  (`KismetSystemLibrary.PrintText` (`KismetTextLibrary.Conv_StringToText` (`KismetStringLibrary.Concat_StrStr` "Rod Angle: " (`KismetStringLibrary.Conv_DoubleToString` (`KismetMathLibrary.RadiansToDegrees` (`Rod.GetAngle` (`self.RodComponent`)))))) true false (struct :`G` 0.66 :`B` 1.0 :`A` 1.0) 0.0))

(event `Key|Q`
  (params (Key :type "Key Structure"))
  (:`Pressed`
    (`CanFall.FallDownTo` (struct))))

(event `Key|R`
  (params (Key :type "Key Structure"))
  (:`Pressed`
    (`self.RespawnRocker` 0.0 "Constrained")))

(event `Key|E`
  (params (Key :type "Key Structure"))
  (:`Pressed`
    (`Rod.ResetLocation` (`self.RodComponent`))))

(event `self.FallDownTo`
  (params (fallDownData :type "FallDownData Structure"))
  (`parent.FallDownTo` fallDownData)
  (`KismetSystemLibrary.PrintText` (`KismetTextLibrary.Conv_StringToText` (`KismetSystemLibrary.GetDisplayName` (`.TargetFallDownTo` (break `FallDownData` fallDownData)))) true true (struct :`G` 0.66 :`B` 1.0 :`A` 1.0) 5.0))

(event `self.ReceivePossessed`
  (params (NewController :type "Controller Object Reference"))
  (bind _asbp_in_game_player_state (cast `/Game/Blueprints/State/BP_InGamePlayerState` (`Controller.PlayerState` NewController)))
  (bind _output_get (set `self.m_InGamePlayerState` _asbp_in_game_player_state))
  (add `InGamePlayerState.OnCurrentLivesCountChanged` _output_get (delegate `ConnectLivesCountEvent`)))

(event `ConnectLivesCountEvent`
  (params (prevLivesCount :type Integer) (newLivesCount :type Integer))
  (`self.HandleOnPlayerStateLivesCountChanged` prevLivesCount newLivesCount))

(event `self.ReceiveBeginPlay`
  (`self.HandleOnPlayerStateLivesCountChanged` 0 (`InGamePlayerState.m_InitialLivesCount` (`self.m_InGamePlayerState`))))

(fn `HandleOnPlayerStateLivesCountChanged`
  (params (prevLivesCount :type Integer) (newLivesCount :type Integer))
  (bind _aswbp_lives_hud (cast `/Game/Blueprints/Widget/WBP_LivesHUD` (`WidgetComponent.GetWidget` (`self.LivesUIWidget`))))
  (`/Game/Blueprints/Widget/WBP_LivesHUD.SetNumberOfEnabledDots` _aswbp_lives_hud newLivesCount))

(fn `InjectReferences`
  (bind _rockercomponent (`self.RockerComponent`))
  (set `self.Rocker` (`self.RockerComponent`))
  (set `self.Rod` (`self.RodComponent`))
  (`Rocker.SetRod` _rockercomponent (`self.RodComponent`))
  (set `Rocker.m_SphereCollision` (`self.SphereCollision`) _rockercomponent)
  (`RodAnimationController.SetRod` (`self.RodAnimationController`) (`self.RodComponent`)))

(fn `OnDrawDebugRocker`
  (locals (delta :type "Float (double-precision)" :default 0.05))
  (bind _sphereradius (`SphereComponent.SphereRadius` (`self.SphereCollision`)))
  (`KismetSystemLibrary.DrawDebugCircle` (+ (+ (`Rod.GetRodCenterLocation` (`self.RodComponent`)) (* (`KismetMathLibrary.Normal` (`Rod.GetRodVector` (`self.RodComponent`))) (`Rocker.m_LocationOnRod` (`self.RockerComponent`)))) (`KismetMathLibrary.MakeVector` 0.0 0.0 _sphereradius)) _sphereradius 20 (struct :`G` 0.016063 :`B` 1.0 :`A` 1.0) (`local.delta`) 1.0 (1.0 0.0 0.0)))

(fn `OnDrawDebugRod`
  (locals (rodCenter :type "Vector Structure" :default (0.0 0.0 0.0)) (centerToRightOriginVector :type "Vector Structure") (rightOrigin :type "Vector Structure") (leftOrigin :type "Vector Structure") (leftMovableRangeUpOffset :type "Vector Structure") (rightMovableRangeUpOffset :type "Vector Structure") (delta :type "Float (double-precision)" :default 0.05))
  (bind _rodcomponent (`self.RodComponent`))
  (bind _returnvalue (`Rod.GetRightEndLocation` (`self.RodComponent`)))
  (bind _returnvalue_2 (`Rod.GetLeftEndLocation` (`self.RodComponent`)))
  ;[1 1 1] Draw Rod Line
  (`KismetSystemLibrary.DrawDebugLine` _returnvalue _returnvalue_2 (struct :`R` 1.0 :`G` 0.86256 :`A` 1.0) (`local.delta`) 1.0)
  (`KismetSystemLibrary.DrawDebugCircle` _returnvalue 2.0 20 (struct :`R` 1.0 :`A` 1.0) (`local.delta`) 1.0 (1.0 0.0 0.0))
  (`KismetSystemLibrary.DrawDebugCircle` _returnvalue_2 2.0 20 (struct :`R` 1.0 :`A` 1.0) (`local.delta`) 1.0 (1.0 0.0 0.0))
  (`KismetSystemLibrary.DrawDebugCircle` (`Rod.GetRodCenterLocation` (`self.RodComponent`)) 5.0 20 (struct :`R` 1.0 :`A` 1.0) (`local.delta`) 1.0 (1.0 0.0 0.0))
  (set `local.rodCenter` (`SceneComponent.K2_GetComponentLocation` _rodcomponent))
  (set `local.centerToRightOriginVector` (* (`SceneComponent.GetForwardVector` _rodcomponent) (`Rod.m_MovableAreaWidth` _rodcomponent) (`KismetMathLibrary.Conv_DoubleToVector` 0.5)))
  (set `local.rightOrigin` (+ (`local.rodCenter`) (`local.centerToRightOriginVector`)))
  (set `local.leftOrigin` (- (`local.rodCenter`) (`local.centerToRightOriginVector`)))
  ;[1 1 1] Draw End Movable Range
  (set `local.leftMovableRangeUpOffset` (* (`KismetMathLibrary.GetUpVector` (struct)) (* (`Rod.m_EndMovableRange` (`self.RodComponent`)) 0.5)))
  (`KismetSystemLibrary.DrawDebugLine` (+ (`local.leftOrigin`) (`local.leftMovableRangeUpOffset`)) (- (`local.leftOrigin`) (`local.leftMovableRangeUpOffset`)) (struct :`G` 0.222723 :`B` 1.0 :`A` 1.0) (`local.delta`) 1.0)
  (set `local.rightMovableRangeUpOffset` (* (`KismetMathLibrary.GetUpVector` (struct)) (* (`Rod.m_EndMovableRange` (`self.RodComponent`)) 0.5)))
  (`KismetSystemLibrary.DrawDebugLine` (+ (`local.rightOrigin`) (`local.rightMovableRangeUpOffset`)) (- (`local.rightOrigin`) (`local.rightMovableRangeUpOffset`)) (struct :`G` 0.222723 :`B` 1.0 :`A` 1.0) (`local.delta`) 1.0))

(fn `UserConstructionScript`
  ;[1 1 1] Connecting Reference
  (`self.InjectReferences`))