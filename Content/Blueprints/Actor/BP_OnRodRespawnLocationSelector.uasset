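; Visual indicator for the on-rod respawn location selector, shown while a player picks where to respawn.
; Selection start reveals outline and fill sprites, pops the sprite group in with a scale tween and plays a sound.
; Tick spins the outline and scales the fill by the player state's Respawning timer progress.
; Selection end hides both sprites and triggers a timer-driven flash sprite that fades from white to transparent.
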(event `self.ReceiveBeginPlay`
  ;[1 1 1] Hide Sprites
  (`SceneComponent.SetVisibility` (`self.OutlineSprite`) false false)
  (`SceneComponent.SetVisibility` (`self.FillSprite`) false false)
  (`SceneComponent.SetVisibility` (`self.FlashSprite`) false false)
  ;[1 1 1] Register Selection Start Event Animation
  (add `self.OnSelectionStart` (delegate `OnSelectionStart_Event_0`))
  (add `TweenComponent.OnTweenUpdate` (`self.OnSelectionStartTween`) (delegate `OnTweenUpdate_Event_0`))
  ;[1 1 1] Register Selection End Event Animation
  (add `self.OnSelectionEnd` (delegate `OnSelectionEnd_Event_0`)))

(event `OnSelectionEnd_Event_0` :!signature `self.OnSelectionEnd`
  (params (locationOnRod :type "Float (single-precision)"))
  ;[1 1 1] Register Selection End Event Animation
  (set `self.m_PlayerState` null)
  (`SceneComponent.SetVisibility` (`self.OutlineSprite`) false false)
  (`SceneComponent.SetVisibility` (`self.FillSprite`) false false)
  (`self.PlayRespawnAnimation`))

(event `OnSelectionStart_Event_0` :!signature `self.OnSelectionStart`
  (params (selectionStartEventData :type "SelectionStartEventData Structure"))
  ;[1 1 1] Register Selection Start Event Animation
  (set `self.m_PlayerState` selectionStartEventData_PlayerState)
  (`SceneComponent.SetRelativeScale3D` (`self.Fill`) (0.0 0.0 0.0))
  (`SceneComponent.SetVisibility` (`self.OutlineSprite`) true false)
  (`SceneComponent.SetVisibility` (`self.FillSprite`) true false)
  (`TweenComponent.Tween` (`self.OnSelectionStartTween`))
  (`GameplayStatics.PlaySound2D` "/Game/Audio/Sfx/SFX_RespawnStart_8Bit.SFX_RespawnStart_8Bit" 1.0 1.0 0.0 null null))

(event `OnTweenUpdate_Event_0`
  (params (progress :type "Float (single-precision)"))
  ;[1 1 1] Register Selection Start Event Animation
  (`self.HandleOnSelectionStartTweenUpdate` progress))

(event `self.ReceiveTick`
  (params (DeltaSeconds :type "Float (single-precision)"))
  (`self.UpdateOutlineRotation` DeltaSeconds)
  (`self.UpdateRespawnAnimation` DeltaSeconds)
  (`self.UpdateFillAnimation` DeltaSeconds))

(fn `HandleOnSelectionStartTweenUpdate`
  (params (progress :type "Float (double-precision)"))
  (`SceneComponent.SetRelativeScale3D` (`self.Location Sprite Group`) (`KismetMathLibrary.Conv_DoubleToVector` progress)))

(fn `PlayRespawnAnimation`
  (`SceneComponent.SetVisibility` (`self.FlashSprite`) true false)
  (`PaperSpriteComponent.SetSpriteColor` (`self.FlashSprite`) (struct :`R` 1.0 :`G` 1.0 :`B` 1.0 :`A` 1.0))
  (set `self.m_IsPlayingRespawnAnimation` true)
  (set `self.m_RespawnAnimationTimer` 0.0))

(fn `StopRespawnAnimation`
  (`SceneComponent.SetVisibility` (`self.FlashSprite`) false false)
  (set `self.m_IsPlayingRespawnAnimation` false))

(fn `UpdateFillAnimation`
  (params (deltaTime :type "Float (double-precision)"))
  (if (`KismetSystemLibrary.IsValid` (`self.m_PlayerState`))
    (if (`|EnumEquality` (`InGamePlayerState.GetGameFlowState` (`self.m_PlayerState`)) "Respawning")
      (`SceneComponent.SetRelativeScale3D` (`self.Fill`) (`KismetMathLibrary.Conv_DoubleToVector` (/ (`InGamePlayerState.GetStateTimer` (`self.m_PlayerState`)) (`InGamePlayerState.m_RespawningTime` (`self.m_PlayerState`))))))))

(fn `UpdateOutlineRotation`
  (params (deltaTime :type "Float (double-precision)"))
  (bind _outlinesprite (`self.OutlineSprite`))
  (`SceneComponent.K2_SetRelativeRotation` _outlinesprite (`KismetMathLibrary.ComposeRotators` (`SceneComponent.RelativeRotation` _outlinesprite) (`KismetMathLibrary.MakeRotator` 0.0 (* deltaTime (`self.m_OutlineAngularSpeed`)))) false false))

(fn `UpdateRespawnAnimation`
  (params (deltaTime :type "Float (double-precision)"))
  (bind _m_respawnanimationtimer (`self.m_RespawnAnimationTimer`))
  (bind _respawnanimationduration (`self.RespawnAnimationDuration`))
  (if (`self.m_IsPlayingRespawnAnimation`)
    (if (<= _m_respawnanimationtimer _respawnanimationduration)
      (bind _output_get (set `self.m_RespawnAnimationTimer` (+ deltaTime _m_respawnanimationtimer)))
      (`PaperSpriteComponent.SetSpriteColor` (`self.FlashSprite`) (`KismetMathLibrary.LinearColorLerp` (struct :`R` 1.0 :`G` 1.0 :`B` 1.0 :`A` 1.0) (struct) (`KismetMathLibrary.FClamp` (/ _output_get _respawnanimationduration))))
      (else
        (`self.StopRespawnAnimation`)))))

(fn `UserConstructionScript`)