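; BP_LifePickUp is a pickup actor that grants an extra life to the player who touches it.
; When its sphere collision overlaps an actor implementing the PickUpUser interface, it calls UsePickUp on that actor with itself.
; For a pawn with a valid InGamePlayerState, it then increments the current lives count and destroys itself.
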(event `self.SphereCollision.OnComponentBeginOverlap`
  (params (OverlappedComponent :type "PrimitiveComponent Object Reference") (OtherActor :type "Actor Object Reference") (OtherComp :type "PrimitiveComponent Object Reference") (OtherBodyIndex :type Integer) (bFromSweep :type Boolean) (SweepResult :type "HitResult Structure (by ref)"))
  (if (`KismetSystemLibrary.DoesImplementInterface` OtherActor "/Script/RollingRocker2D.PickUpUser")
    (bind _aspick_up_user (cast `PickUpUser` OtherActor))
    (`PickUpUser.UsePickUp` _aspick_up_user (make `PickUpData` self))
    (bind _aspawn (cast `Pawn` OtherActor))
    (bind _playerstate (`Pawn.PlayerState` _aspawn))
    (if (`KismetSystemLibrary.IsValid` _playerstate)
      (bind _asin_game_player_state (cast `InGamePlayerState` _playerstate))
      (`InGamePlayerState.SetCurrentLivesCount` _asin_game_player_state (+ (`InGamePlayerState.m_CurrentLivesCount` _asin_game_player_state) 1))
      (`self.K2_DestroyActor`))))

(fn `UserConstructionScript`)