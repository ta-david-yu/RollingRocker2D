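; BP_BgmManager adjusts the background music to match the game's paused or playing state.
; On BeginPlay it casts player controller 0 to InGamePlayerController and binds to its OnPaused and OnResumed events.
; Pausing halves the BackgroundMusicAudio volume multiplier and enables its low-pass filter for a muffled sound, while resuming restores full volume and disables the filter.
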(event `self.ReceiveBeginPlay`
  (bind _asin_game_player_controller (cast `InGamePlayerController` (`GameplayStatics.GetPlayerController` 0)))
  (add `InGamePlayerController.OnPaused` _asin_game_player_controller (delegate `OnPaused_Event_0`))
  (add `InGamePlayerController.OnResumed` _asin_game_player_controller (delegate `OnResumed_Event_0`)))

(event `OnPaused_Event_0`
  (`self.ApplyPauseModeSettings`))

(event `OnResumed_Event_0`
  (`self.ApplyPlayModeSettings`))

(fn `ApplyPauseModeSettings`
  (`AudioComponent.SetVolumeMultiplier` (`self.Background Music Audio`) 0.5)
  (`AudioComponent.SetLowPassFilterEnabled` (`self.Background Music Audio`) true))

(fn `ApplyPlayModeSettings`
  (`AudioComponent.SetVolumeMultiplier` (`self.Background Music Audio`) 1.0)
  (`AudioComponent.SetLowPassFilterEnabled` (`self.Background Music Audio`) false))

(fn `UserConstructionScript`)